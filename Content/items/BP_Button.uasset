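; BP_Button is a level-exit button actor that loads the level named in NextLevel when anything begins overlapping its Sphere component.
; On overlap, MoveComponentTo lowers the Button component by three units and then raises it back, with a short delay before each move, before opening the level.
; The overlap is not filtered by actor type.
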(event `self.Sphere.OnComponentBeginOverlap`
  (params (OverlappedComponent :type "PrimitiveComponent Object Reference") (OtherActor :type "Actor Object Reference") (OtherComp :type "PrimitiveComponent Object Reference") (OtherBodyIndex :type Integer) (bFromSweep :type Boolean) (SweepResult :type "HitResult Structure (by ref)"))
  (bind _button (`self.button`))
  (bind _button_2 (`self.button`))
  (bind (_returnvalue_location _returnvalue_rotation) (`KismetMathLibrary.BreakTransform` (`SceneComponent.GetRelativeTransform` _button)))
  (bind (_returnvalue_location_2 _returnvalue_rotation_2) (`KismetMathLibrary.BreakTransform` (`SceneComponent.GetRelativeTransform` _button_2)))
  (`KismetSystemLibrary.Delay` 0.2) ; Задержка\\пауза
  (`KismetSystemLibrary.MoveComponentTo` _button_2 (+ _returnvalue_location_2 (0.0 0.0 -3.0)) _returnvalue_rotation_2) ; Передвижение обьекта
  (`KismetSystemLibrary.Delay` 0.2) ; Задержка\\пауза
  (`KismetSystemLibrary.MoveComponentTo` _button (+ _returnvalue_location (0.0 0.0 3.0)) _returnvalue_rotation) ; Передвижение обьекта
  (`GameplayStatics.OpenLevel` (`self.NextLevel`)))

(fn `UserConstructionScript`)